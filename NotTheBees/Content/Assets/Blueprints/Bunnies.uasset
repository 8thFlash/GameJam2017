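; Bunny actor that walks in a straight line toward a point it is attracted to.
; Attract sets a normalized walk direction toward the given location and enables walking.
; While walking is enabled, Tick moves it by that direction each frame with a swept location change, independent of delta time.
; Hits from anything other than exactly ThirdPersonCharacter also enable walking, and nothing in this graph turns it off.
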(event `self.ReceiveHit`
  (params (MyComp :type "PrimitiveComponent Object Reference") (Other :type "Actor Object Reference") (OtherComp :type "PrimitiveComponent Object Reference") (bSelfMoved :type Boolean) (HitLocation :type "Vector Structure") (HitNormal :type "Vector Structure") (NormalImpulse :type "Vector Structure") (Hit :type "HitResult Structure (by ref)"))
  (if (not (== (`GameplayStatics.GetObjectClass` Other) "/Game/ThirdPersonBP/Blueprints/ThirdPersonCharacter.ThirdPersonCharacter_C"))
    (set `self.CanWalk` true)))

(event `Walk`
  (`self.K2_SetActorLocation` (+ (`self.K2_GetActorLocation`) (`self.WalkDir`)) true))

(event `self.ReceiveTick`
  (params (DeltaSeconds :type "Float (single-precision)"))
  (if (`self.CanWalk`)
    (`self.Walk`)))

(event `Attract`
  (params (OtherDir :type "Vector Structure"))
  (set `self.WalkDir` (`KismetMathLibrary.Normal` (- OtherDir (`self.K2_GetActorLocation`))))
  (set `self.CanWalk` true))

(fn `UserConstructionScript`)